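; Registration actor that adds the FLAGS mod's built-in textures to the FLAGS_ADDON_MANAGER on BeginPlay.
; It records named, credited categories for 2x1 (FLAGS Default and FICSIT), 1x1 and stacked 2x1 textures, then appends its own texture lists to the manager's shared arrays.
; Each category's start index is the target array's length before appending.
; The actor destroys itself once registration finishes.
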(event EventBeginPlay
  (bind _outactors (Actor|GetAllActorsOfClass "/Game/FLAGSMod/Blueprints/FLAGS_ADDON_MANAGER.FLAGS_ADDON_MANAGER_C"))
  (Utilities|FlowControl|Sequence
    (:then_0
      (Utilities|Array|Add (Variables|/Game/FLAGSMod/Blueprints/FLAGS_ADDON_MANAGER.FLAGS_ADDON_MANAGER_C|Get2x1%20Texture%20Cats (Utilities|Array|Get(acopy) _outactors)) (Utilities|Struct|MakeTextureCat_Struct (Utilities|Array|Length (Variables|/Game/FLAGSMod/Blueprints/FLAGS_ADDON_MANAGER.FLAGS_ADDON_MANAGER_C|Get2x1%20Texture%20Array (Utilities|Array|Get(acopy) _outactors))) "FLAGS Default" "Illya & Dean"))
      (for _array_element (Variables|Default|Get2x1%20Misc%20Textures)
        (Utilities|Array|Add (Variables|/Game/FLAGSMod/Blueprints/FLAGS_ADDON_MANAGER.FLAGS_ADDON_MANAGER_C|Get2x1%20Texture%20Array (Utilities|Array|Get(acopy) _outactors)) _array_element)))
    (:then_1
      (Utilities|Array|Add (Variables|/Game/FLAGSMod/Blueprints/FLAGS_ADDON_MANAGER.FLAGS_ADDON_MANAGER_C|Get2x1%20Texture%20Cats (Utilities|Array|Get(acopy) _outactors)) (Utilities|Struct|MakeTextureCat_Struct (Utilities|Array|Length (Variables|/Game/FLAGSMod/Blueprints/FLAGS_ADDON_MANAGER.FLAGS_ADDON_MANAGER_C|Get2x1%20Texture%20Array (Utilities|Array|Get(acopy) _outactors))) "FICSIT" "Illya & Dean"))
      (for _array_element_2 (Variables|Default|Get2x1%20FICSIT%20Textures)
        (Utilities|Array|Add (Variables|/Game/FLAGSMod/Blueprints/FLAGS_ADDON_MANAGER.FLAGS_ADDON_MANAGER_C|Get2x1%20Texture%20Array (Utilities|Array|Get(acopy) _outactors)) _array_element_2)))
    (:then_2
      (Utilities|Array|Add (Variables|/Game/FLAGSMod/Blueprints/FLAGS_ADDON_MANAGER.FLAGS_ADDON_MANAGER_C|Get1x1%20Texture%20Cats (Utilities|Array|Get(acopy) _outactors)) (Utilities|Struct|MakeTextureCat_Struct (Utilities|Array|Length (Variables|/Game/FLAGSMod/Blueprints/FLAGS_ADDON_MANAGER.FLAGS_ADDON_MANAGER_C|Get1x1%20Texture%20Array (Utilities|Array|Get(acopy) _outactors))) "FLAGS Default" "Illya & Dean"))
      (for _array_element_3 (Variables|Default|Get1x1%20Default%20Textures)
        (Utilities|Array|Add (Variables|/Game/FLAGSMod/Blueprints/FLAGS_ADDON_MANAGER.FLAGS_ADDON_MANAGER_C|Get1x1%20Texture%20Array (Utilities|Array|Get(acopy) _outactors)) _array_element_3)))
    (:then_3
      (Utilities|Array|Add (Variables|/Game/FLAGSMod/Blueprints/FLAGS_ADDON_MANAGER.FLAGS_ADDON_MANAGER_C|GetStacked%202x1%20Texture%20Cats (Utilities|Array|Get(acopy) _outactors)) (Utilities|Struct|MakeTextureCat_Struct (Utilities|Array|Length (Variables|/Game/FLAGSMod/Blueprints/FLAGS_ADDON_MANAGER.FLAGS_ADDON_MANAGER_C|GetStacked%202x1%20Texture%20Array (Utilities|Array|Get(acopy) _outactors))) "FLAGS Default" "Illya & Dean"))
      (for _array_element_4 (Variables|Default|GetStacked%202x1%20Default%20Textures)
        (Utilities|Array|Add (Variables|/Game/FLAGSMod/Blueprints/FLAGS_ADDON_MANAGER.FLAGS_ADDON_MANAGER_C|GetStacked%202x1%20Texture%20Array (Utilities|Array|Get(acopy) _outactors)) _array_element_4)))
    (:then_4
      (Actor|DestroyActor))))

(fn ConstructionScript)